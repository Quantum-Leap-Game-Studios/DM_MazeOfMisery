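; BP_NPC_Guardian is a guardian NPC that the player can talk to.
; Its box trigger shows an interaction widget when the HorrorEngineCharacter enters and removes it when an overlap ends.
; The Speak event removes that prompt and creates a subtitle widget, which plays either the whole Dialogue array or one random line from it, depending on the Test flag.
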(event `self.Box.OnComponentBeginOverlap`
  (params (OverlappedComponent :type "PrimitiveComponent Object Reference") (OtherActor :type "Actor Object Reference") (OtherComp :type "PrimitiveComponent Object Reference") (OtherBodyIndex :type Integer) (bFromSweep :type Boolean) (SweepResult :type "HitResult Structure (by ref)"))
  (cast `/Game/HorrorEngine/Blueprints/Core/HorrorEngineCharacter` OtherActor)
  (bind _returnvalue (`|CreateWidget` "/Game/Blueprints/Widgets/Components/WBP_NPC_Interaction.WBP_NPC_Interaction_C"))
  (`UserWidget.AddToViewport` _returnvalue 0)
  (set `self.Widget` _returnvalue))

(event `self.Box.OnComponentEndOverlap`
  (params (OverlappedComponent :type "PrimitiveComponent Object Reference") (OtherActor :type "Actor Object Reference") (OtherComp :type "PrimitiveComponent Object Reference") (OtherBodyIndex :type Integer))
  (`Widget.RemoveFromParent` (`self.Widget`)))

(event `/Game/Blueprints/Actors/NPC/BPI_NPC_Interface.Speak`
  (`Widget.RemoveFromParent` (`self.Widget`))
  (if (`self.test?`)
    (bind _returnvalue (`|CreateWidget` "/Game/Blueprints/Widgets/Components/WBP_SubtitleNPC.WBP_SubtitleNPC_C"))
    (`UserWidget.AddToViewport` _returnvalue 0)
    (`/Game/Blueprints/Widgets/Components/WBP_SubtitleNPC.PlaySubtitle` _returnvalue (`self.Dialogue`) 3.0)
    (else
      (bind _returnvalue_2 (`|CreateWidget` "/Game/Blueprints/Widgets/Components/WBP_SubtitleNPC.WBP_SubtitleNPC_C"))
      (`UserWidget.AddToViewport` _returnvalue_2 0)
      (`/Game/Blueprints/Widgets/Components/WBP_SubtitleNPC.PlaySubtitle` _returnvalue_2 (`|MakeArray` (`KismetArrayLibrary.Array_Random` (`self.Dialogue`))) 4.0))))

(fn `UserConstructionScript`)