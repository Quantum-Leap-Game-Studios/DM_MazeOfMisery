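; BP_HUD_Menu is the menu HUD that switches between main menu, settings, mode selection, hosting and joining screens.
; The construction script pre-creates one widget per E_HUD_Menu entry, cached in a class-keyed map.
; BeginPlay displays the first screen with its appear animation.
; ChangeWidget logs the transition and starts the current screen's disappearance, whose finish callback removes it and displays the pending screen.
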(event `self.ReceiveBeginPlay`
  (`self.DisplayWidget` "NewEnumerator0"))

(event `/Game/Blueprints/Core/BPI_HUD_Menu.ChangeWidget`
  (params (Widget :type "/Game/Blueprints/Core/E_HUD_Menu Enum" :default "NewEnumerator0"))
  (set `self.NextWidget` Widget)
  (`/Game/Blueprints/Libraries/BPLF_Global.Print` "NewEnumerator2" (`KismetStringLibrary.Concat_StrStr` "From [" (`|GetEnumeratorNameAsString` (`self.CurrentWidget`)) "] to [" (`|GetEnumeratorNameAsString` (`self.NextWidget`)) "]"))
  (`self.RemoveWidget` (`self.CurrentWidget`)))

(fn `DisplayWidget`
  (params (WidgetToDisplay :type "/Game/Blueprints/Core/E_HUD_Menu Enum" :default "NewEnumerator0"))
  (bind _widget (`self.GetWidget` WidgetToDisplay))
  (`UserWidget.AddToViewport` _widget 0)
  (`/Game/Blueprints/Widgets/Core/WBP_UserWidget.AppearBegin` _widget)
  (bind _output_get (set `self.CurrentWidget` WidgetToDisplay))
  (set `self.NextWidget` _output_get))

(fn `GetWidget`
  (params (Type :type "/Game/Blueprints/Core/E_HUD_Menu Enum" :default "NewEnumerator0"))
  (returns (Widget :type "/Game/Blueprints/Widgets/Core/WBP_UserWidget Object Reference"))
  (return (`BlueprintMapLibrary.Map_Find` (`self.ListWidgets`) (`|GetArrayItem` (`|MakeArray` "/Game/Blueprints/Widgets/WBP_MainMenu.WBP_MainMenu_C" "/Game/Blueprints/Widgets/Settings/WBP_Settings.WBP_Settings_C" "/Game/Blueprints/Widgets/Play/WBP_ModeSelection.WBP_ModeSelection_C" "/Game/Blueprints/Widgets/Play/WBP_Hosting.WBP_Hosting_C" "/Game/Blueprints/Widgets/Play/WBP_Joining.WBP_Joining_C" :!type "/Game/Blueprints/Widgets/Core/WBP_UserWidget Class Reference") (`KismetMathLibrary.Conv_ByteToInt` Type)))))

(fn `OnDisappearFinsh`
  (params (Widget :type "/Game/Blueprints/Widgets/Core/WBP_UserWidget Object Reference"))
  (`Widget.RemoveFromParent` Widget)
  (if (`|EnumInequality` (`self.CurrentWidget`) (`self.NextWidget`))
    (`self.DisplayWidget` (`self.NextWidget`))))

(fn `RemoveWidget`
  (params (WidgetToRemove :type "/Game/Blueprints/Core/E_HUD_Menu Enum" :default "NewEnumerator0"))
  (bind _widget (`self.GetWidget` WidgetToRemove))
  (add `/Game/Blueprints/Widgets/Core/WBP_UserWidget.DisapearFinish` _widget (`|CreateDelegate` :!event `OnDisappearFinsh`))
  (`/Game/Blueprints/Widgets/Core/WBP_UserWidget.DisappearBegin` _widget))

(fn `UserConstructionScript`
  (`self.SetupDefaultWidgets`))