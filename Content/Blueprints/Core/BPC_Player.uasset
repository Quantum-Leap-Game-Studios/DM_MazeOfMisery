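; Player controller for a networked two-player game, handling input setup, text chat and guest username entry.
; On local BeginPlay it applies saved keybind and control mapping contexts and creates the chat panel, which Enter focuses.
; Key presses and mouse movement track controller use, toggling the cursor while nav-list widgets are shown.
; Interface events route to server and client events that relay chat to all players, prompt for usernames and label both characters.
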(event `UpdateMapping`
  (bind _returnvalue (pcsubsystem `EnhancedInputLocalPlayerSubsystem` self))
  (bind ((`Keybinds_9_7953C22E4C20CB214354E4967FCB2862` _keybinds) (`Controls_19_42AECADE486D131CA681088243FE3EDC` _controls)) (break `/Game/Classes/Structures/Settings/S_Settings` (`/Game/Saves/BP_SaveGame.Settings` (`/Game/Blueprints/Core/GI_Global.SaveGame` (`self.GameInstanceRef`)))))
  ;[1 1 1] Mapping | Keyboard/Controller
  (if (`self.IsLocalPlayerController`)
    (`EnhancedInputSubsystemInterface.ClearAllMappings` _returnvalue)
    (`EnhancedInputSubsystemInterface.AddMappingContext` _returnvalue (`.MappingContext_47_CDC411FF4FBB38A1C82E40B1097133EF` (break `/Game/Classes/Structures/Settings/S_KeybindsSettings` _keybinds)) 0 (struct))
    (`EnhancedInputSubsystemInterface.AddMappingContext` _returnvalue (`.MappingContext_47_CDC411FF4FBB38A1C82E40B1097133EF` (break `/Game/Classes/Structures/Settings/S_ControlsSettings` _controls)) 0 (struct))))

(event `Key|AnyKey` :paused true
  (params (Key :type "Key Structure"))
  ;[1 1 1] Mapping | Keyboard/Controller
  ;;[0.588 1 0] Controller Check
  (:`Pressed`
    (`self.HandleKeyPressed` Key)
    (bind _foundwidgets (`WidgetBlueprintLibrary.GetAllWidgetsOfClass` "/Game/Blueprints/Widgets/Core/WBP_NavList.WBP_NavList_C" :!label _label))
    (if (`KismetArrayLibrary.Array_IsNotEmpty` _foundwidgets)
      (set `self.bShowMouseCursor` (not (`self.ControllerConnected?`))))))

(event `self.ReceiveTick`
  (params (DeltaSeconds :type "Float (single-precision)"))
  ;[1 1 1] Mapping | Keyboard/Controller
  ;;[0.588 1 0] Controller Check
  (`self.HandleMouseMoved`)
  (goto _label))

(event `self.ReceiveBeginPlay`
  (if (`self.IsLocalPlayerController`)
    (`|ExecutionSequence`
      (:`then_0`
        (bind _asgi_global (cast `/Game/Blueprints/Core/GI_Global` (`GameplayStatics.GetGameInstance`))
          (:`then`
            (set `self.GameInstanceRef` _asgi_global)
            (`self.UpdateMapping`))
          (:`CastFailed`
            (`/Game/Blueprints/Libraries/BPLF_Global.Print` "NewEnumerator0" "Game Instance failed"))))
      (:`then_1`
        (bind _returnvalue (`|CreateWidget` "/Game/Blueprints/Widgets/Chat/WBP_ChatPanel.WBP_ChatPanel_C" self))
        (bind _output_get (set `self.ChatRef` _returnvalue))
        (`UserWidget.AddToViewport` _output_get 0)))))

(event `Key|Enter`
  (params (Key :type "Key Structure"))
  ;[1 1 1] Chat
  (:`Pressed`
    (bind _chatref (`self.ChatRef`)
      (:`then`
        (`Widget.SetKeyboardFocus` (`/Game/Blueprints/Widgets/Chat/WBP_ChatPanel.Chat_TextBox` _chatref)))
      (:`else`))))

(event `CLI_AskUsername`
  ;[1 1 1] Username
  (bind _returnvalue (`|CreateWidget` "/Game/Blueprints/Widgets/Components/WBP_AskUsername.WBP_AskUsername_C" self))
  (`UserWidget.AddToViewport` _returnvalue 0)
  (`WidgetBlueprintLibrary.SetInputMode_GameAndUIEx` self _returnvalue)
  (set `self.bShowMouseCursor` true))

(event `SR_SubmitChat`
  (params (PlayerName :type Text) (ChatMessage :type Text))
  ;[1 1 1] Chat
  (for _array_element (`GameStateBase.PlayerArray` (`GameplayStatics.GetGameState`))
    (message `/Game/Blueprints/Interfaces/BPI_PC_Events.SubmitChat` (`PlayerState.GetPlayerController` _array_element) false PlayerName ChatMessage)))

(event `SR_AskUsernameFinish`
  ;[1 1 1] Username
  (message `/Game/Blueprints/Interfaces/BPI_GM_Events.GuestUsernameHasBeenSet` (`GameplayStatics.GetGameMode`)))

(event `CLI_SetCharactersNames`
  (params (`Player1 Name` :type Text) (`Player2 Name` :type Text))
  ;[1 1 1] Username
  (bind (_player_1 _player_2) (`self.GetPlayersCharacters`)
    (:`Success`
      (message `/Game/Blueprints/Interfaces/BPI_Character.UpdateName` _player_1 `Player1 Name`)
      (message `/Game/Blueprints/Interfaces/BPI_Character.UpdateName` _player_2 `Player2 Name`))
    (:`Failed`
      (`/Game/Blueprints/Libraries/BPLF_Global.Print` "NewEnumerator0" "Get 2 HE Characters failed"))))

(event `CLI_SubmitChat`
  (params (PlayerName :type Text) (ChatMessage :type Text))
  ;[1 1 1] Chat
  (bind _chatref (`self.ChatRef`)
    (:`then`
      (`/Game/Blueprints/Widgets/Chat/WBP_ChatPanel.UpdateChat` _chatref PlayerName ChatMessage))
    (:`else`)))

(event `/Game/Blueprints/Interfaces/BPI_PC_Events.AskUsername`
  ;[1 1 1] Guest Username
  (`self.CLI_AskUsername`))

(event `/Game/Blueprints/Interfaces/BPI_PC_Events.SetCharactersNames`
  (params (`Player1 Name` :type Text) (`Player2 Name` :type Text))
  ;[1 1 1] Guest Username
  (`self.CLI_SetCharactersNames` `Player1 Name` `Player2 Name`)
  (`/Game/Blueprints/Libraries/BPLF_Global.Print` "NewEnumerator1" (`KismetStringLibrary.Concat_StrStr` (`KismetTextLibrary.Conv_TextToString` `Player1 Name`) " - " (`KismetTextLibrary.Conv_TextToString` `Player2 Name`))))

(event `/Game/Blueprints/Interfaces/BPI_PC_Events.AskUsernameFinish`
  ;[1 1 1] Guest Username
  (`self.SR_AskUsernameFinish`))

(event `/Game/Blueprints/Interfaces/BPI_PC_Events.SubmitChat`
  (params (`OnServer?` :type Boolean) (PlayerName :type Text) (ChatMessage :type Text))
  ;[1 1 1] Chat
  (if `OnServer?`
    (`self.SR_SubmitChat` PlayerName ChatMessage)
    (else
      (`self.CLI_SubmitChat` PlayerName ChatMessage))))

(fn `AddNavigationMapping`
  (`EnhancedInputSubsystemInterface.AddMappingContext` (pcsubsystem `EnhancedInputLocalPlayerSubsystem` (`GameplayStatics.GetPlayerController` 0)) "/Game/Inputs/IMC_ControllerNavigation.IMC_ControllerNavigation" 0 (struct))
  (return))

(fn `UserConstructionScript`)