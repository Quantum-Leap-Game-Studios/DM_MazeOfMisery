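; BP_CellDoor is a sliding prison cell door actor that opens by itself shortly after play begins.
; On BeginPlay it stores the Door component's relative transform, waits briefly, then calls OpenDoor.
; OpenDoor plays a timeline that lerps a Y offset from the stored position, sliding the door along its local axis while keeping rotation and scale.
; There is no closing logic or interaction trigger.
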(event `self.ReceiveBeginPlay`
  (set `self.Postition` (`SceneComponent.GetRelativeTransform` (`self.Door`)))
  (`KismetSystemLibrary.Delay` 1.0)
  (`self.Open Door`))

(event `Open Door`
  (bind _postition (`self.Postition`))
  (bind (_direction _transition) (`Timeline|OpentDoorTL` :!via `PlayFromStart`)
    (:`Update`
      (`SceneComponent.K2_SetRelativeTransform` (`self.Door`) (`KismetMathLibrary.MakeTransform` (`KismetMathLibrary.MakeVector` (.x (.location _postition)) (- (.y (.location _postition)) (`KismetMathLibrary.Lerp` 0.0 176.0 _transition)) (.z (.location _postition))) (.rotation _postition) (.scale _postition)) false false))))

(fn `UserConstructionScript`)