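; Game HUD that manages which menu widget is on screen, such as Pause or Settings, selected through the E_HUD_Menu enum.
; The construction script pre-creates the widgets into a class-keyed map, with the first enum-to-class slot deliberately left empty.
; ChangeWidget logs the switch and starts the current widget's disappear sequence.
; Its finish callback removes that widget, then displays the pending one with its appear sequence; an invalid current widget skips straight to this step.
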(event `self.ReceiveBeginPlay`
  (`self.DisplayWidget` "NewEnumerator6"))

(event `/Game/Blueprints/Core/BPI_HUD_Game.ChangeWidget`
  (params (Widget :type "/Game/Blueprints/Core/E_HUD_Game Enum" :default "NewEnumerator6"))
  (set `self.NextWidget` Widget)
  (`/Game/Blueprints/Libraries/BPLF_Global.Print` "NewEnumerator2" (`KismetStringLibrary.Concat_StrStr` "From [" (`|GetEnumeratorNameAsString` (`self.CurrentWidget`)) "] to [" (`|GetEnumeratorNameAsString` (`self.NextWidget`)) "]"))
  (`self.RemoveWidget` (`self.CurrentWidget`)))

(fn `DisplayWidget`
  (params (WidgetToDisplay :type "/Game/Blueprints/Core/E_HUD_Game Enum" :default "NewEnumerator6"))
  (bind _widget (`self.GetWidget` WidgetToDisplay))
  (`/Engine/EditorBlueprintResources/StandardMacros.IsValid` _widget
    (:`Is Valid`
      (`UserWidget.AddToViewport` _widget 0)
      (`/Game/Blueprints/Widgets/Core/WBP_UserWidget.AppearBegin` _widget))
    (:`Is Not Valid`
      _))
  (bind _output_get (set `self.CurrentWidget` WidgetToDisplay))
  (set `self.NextWidget` _output_get))

(fn `GetCurrentWidget`
  (returns (Widget :type "/Game/Blueprints/Widgets/Core/WBP_UserWidget Object Reference"))
  (return (`self.GetWidget` (`self.CurrentWidget`))))

(fn `GetWidget`
  (params (Type :type "/Game/Blueprints/Core/E_HUD_Game Enum" :default "NewEnumerator6"))
  (returns (Widget :type "/Game/Blueprints/Widgets/Core/WBP_UserWidget Object Reference"))
  (return (`BlueprintMapLibrary.Map_Find` (`self.ListWidgets`) (`|GetArrayItem` (`|MakeArray` null "/Game/Blueprints/Widgets/WBP_Pause.WBP_Pause_C" "/Game/Blueprints/Widgets/Settings/WBP_Settings.WBP_Settings_C" :!type "/Game/Blueprints/Widgets/Core/WBP_UserWidget Class Reference") (`KismetMathLibrary.Conv_ByteToInt` Type)))))

(fn `OnDisappearFinsh`
  (params (Widget :type "/Game/Blueprints/Widgets/Core/WBP_UserWidget Object Reference"))
  (`/Engine/EditorBlueprintResources/StandardMacros.IsValid` Widget
    (:`Is Valid`
      (`Widget.RemoveFromParent` Widget))
    (:`Is Not Valid`
      _))
  (if (`|EnumInequality` (`self.CurrentWidget`) (`self.NextWidget`))
    (`self.DisplayWidget` (`self.NextWidget`))))

(fn `RemoveWidget`
  (params (WidgetToRemove :type "/Game/Blueprints/Core/E_HUD_Game Enum" :default "NewEnumerator6"))
  (bind _widget (`self.GetWidget` WidgetToRemove))
  (`/Engine/EditorBlueprintResources/StandardMacros.IsValid` _widget
    (:`Is Valid`
      (add `/Game/Blueprints/Widgets/Core/WBP_UserWidget.DisapearFinish` _widget (`|CreateDelegate` :!event `OnDisappearFinsh`))
      (`/Game/Blueprints/Widgets/Core/WBP_UserWidget.DisappearBegin` _widget))
    (:`Is Not Valid`
      (`self.OnDisappearFinsh` _widget))))

(fn `UserConstructionScript`
  (`self.SetupDefaultWidgets`))