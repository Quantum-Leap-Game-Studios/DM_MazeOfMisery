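; Global Game Instance that owns the game's save object and provides Save and Load events.
; Init creates a fresh BP_SaveGame, whose own slot name and user index determine where data is written and read.
; Load replaces that object with the one from the slot if a save exists.
; Both events print the outcome as an on-screen or log message through a typed Print helper.
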(event `self.ReceiveInit`
  (bind _returnvalue (`GameplayStatics.CreateSaveGameObject` "/Game/Saves/BP_SaveGame.BP_SaveGame_C"))
  (set `self.SaveGame` _returnvalue))

(event `Load`
  (bind _savegame (`self.SaveGame`))
  (bind _saveslotname (`/Game/Saves/BP_SaveGame.SaveSlotName` _savegame))
  (bind _userindex (`/Game/Saves/BP_SaveGame.UserIndex` _savegame))
  ;[0 1 0.281 1 24] Save/Load game
  (bind _returnvalue (`GameplayStatics.DoesSaveGameExist` _saveslotname _userindex))
  (if _returnvalue
    (bind _returnvalue_2 (`GameplayStatics.LoadGameFromSlot` _saveslotname _userindex))
    (bind _asbp_save_game (cast `/Game/Saves/BP_SaveGame` _returnvalue_2))
    (set `self.SaveGame` _asbp_save_game)
    (`/Game/Blueprints/Libraries/BPLF_Global.Print` "NewEnumerator4" "[GameInstance] - Game have been loaded successfully")
    (else
      (`/Game/Blueprints/Libraries/BPLF_Global.Print` "NewEnumerator0" (`KismetStringLibrary.Concat_StrStr` "[GameInstance] - No save at slot named : " _saveslotname)))))

(event `Save`
  (bind _savegame (`self.SaveGame`))
  ;[0 1 0.281 1 24] Save/Load game
  (bind _returnvalue (`GameplayStatics.SaveGameToSlot` _savegame (`/Game/Saves/BP_SaveGame.SaveSlotName` _savegame) (`/Game/Saves/BP_SaveGame.UserIndex` _savegame)))
  (if _returnvalue
    (`/Game/Blueprints/Libraries/BPLF_Global.Print` "NewEnumerator4" "[GameInstance] - Game have been saved successfully")
    (else
      (`/Game/Blueprints/Libraries/BPLF_Global.Print` "NewEnumerator0" "[GameInstance] - Game haven't been Saved "))))