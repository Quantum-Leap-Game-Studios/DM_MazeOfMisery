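; Menu manager actor that creates the main menu, settings and blurred background widgets and switches between them with animations, opening on the main menu.
; Widgets live in a map keyed by names parsed from their display names and can request changes through a bound event.
; ChangeWidget handles the blur, then sequences disappear and appear animations by polling a running flag cleared by finish callbacks, before notifying every widget.
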(event `self.ReceiveBeginPlay`
  (`self.CreateMenuWidgets`)
  (bind _values (`BlueprintMapLibrary.Map_Values` (`self.Widgets`)))
  (add `/Game/Blueprints/Widgets/Core/WBP_UserWidget.ChangeWidget` _values (`|CreateDelegate` :!event `ChangeWidget`))
  (`self.ChangeWidget` "MainMenu"))

(event `ChangeWidget`
  (params (`New Widget` :type String) (`NeedBlurredBackground?` :type Boolean))
  (`/Game/Blueprints/Widgets/Core/WBP_UserWidget.OnWidgetChangeBegin` (`BlueprintMapLibrary.Map_Find` (`self.Widgets`) `New Widget`))
  (`self.HandleBlurredBackground` `NeedBlurredBackground?`)
  (`self.RemoveWidget(WithAnim)` (`self.CurrentWidget`))
  (`self.WaitBoolTrue` (`self.AnimationRunning?`))
  (bind _output_get (set `self.CurrentWidget` `New Widget`))
  (`self.DisplayWidget(WithAnim)` _output_get)
  (`self.WaitBoolTrue` (`self.AnimationRunning?`))
  (`self.HandleWidgetChange`))

(event `ResetAnimRunning`
  ;[0 0 0] Event for finish animations
  (set `self.AnimationRunning?` false))

(event `DisableWidget`
  (params (Widget :type "/Game/Blueprints/Widgets/Core/WBP_UserWidget Object Reference"))
  ;[0 0 0] Event for finish animations
  (`self.ResetAnimRunning`)
  (`/Game/Blueprints/Libraries/BPLF_Global.DisplayWidget` Widget)
  (`self.UnbindAllFinishAnim` Widget)
  (`/Game/Blueprints/Libraries/BPLF_Global.Print` "NewEnumerator4" "FINISH ANIM"))

(event `RemoveWidget(WithAnim)`
  (params (Widget :type String))
  (bind (_value _returnvalue) (`BlueprintMapLibrary.Map_Find` (`self.Widgets`) Widget))
  ;[0 1 0] Handle Appear/Disappear widget
  (if _returnvalue
    (`/Game/Blueprints/Widgets/Core/WBP_UserWidget.DisappearBegin` _value)
    (set `self.AnimationRunning?` true)
    (add `/Game/Blueprints/Widgets/Core/WBP_UserWidget.DisapearFinish` _value (`|CreateDelegate` :!event `DisableWidget`))
    (else
      (`/Game/Blueprints/Libraries/BPLF_Global.Print` "NewEnumerator0" "Do not find widget"))))

(event `DisplayWidget(WithAnim)`
  (params (Widget :type String))
  (bind (_value _returnvalue) (`BlueprintMapLibrary.Map_Find` (`self.Widgets`) Widget))
  ;[0 1 0] Handle Appear/Disappear widget
  (if _returnvalue
    (`/Game/Blueprints/Libraries/BPLF_Global.DisplayWidget` _value true)
    (`/Game/Blueprints/Widgets/Core/WBP_UserWidget.AppearBegin` _value)
    (set `self.AnimationRunning?` true)
    (add `/Game/Blueprints/Widgets/Core/WBP_UserWidget.AppearFinish` _value (`|CreateDelegate` :!event `ResetAnimRunning`))
    (else
      (`/Game/Blueprints/Libraries/BPLF_Global.Print` "NewEnumerator0" "Do not find widget"))))

(fn `CreateMenuWidgets`
  (`BlueprintMapLibrary.Map_Clear` (`self.Widgets`))
  (`|ExecutionSequence`
    (:`then_0`
      (bind _returnvalue (`|CreateWidget` "/Game/Blueprints/Widgets/WBP_MainMenu.WBP_MainMenu_C"))
      (`BlueprintMapLibrary.Map_Add` (`self.Widgets`) (`self.GetWidgetName` _returnvalue) _returnvalue))
    (:`then_1`
      (bind _returnvalue_2 (`|CreateWidget` "/Game/Blueprints/Widgets/Settings/WBP_Settings.WBP_Settings_C"))
      (`BlueprintMapLibrary.Map_Add` (`self.Widgets`) (`self.GetWidgetName` _returnvalue_2) _returnvalue_2))
    (:`then_2`
      (bind _returnvalue_3 (`|CreateWidget` "/Game/Blueprints/Widgets/Components/WBP_BackgroundBlurred.WBP_BackgroundBlurred_C" null true))
      (`BlueprintMapLibrary.Map_Add` (`self.Widgets`) (`self.GetWidgetName` _returnvalue_3) _returnvalue_3))
    (:`then_3`
      (return))))

(fn `GetWidgetName`
  (params (Object :type "Object Object Reference"))
  (returns (String :type String))
  (return (`KismetStringLibrary.Split` (`.RightS` (`KismetStringLibrary.Split` (`KismetSystemLibrary.GetDisplayName` Object) "_")) "_")))

(fn `HandleWidgetChange`
  (bind _values (`BlueprintMapLibrary.Map_Values` (`self.Widgets`)))
  (for _array_element _values
    (`/Game/Blueprints/Widgets/Core/WBP_UserWidget.OnWidgetChangeFinish` _array_element (`KismetStringLibrary.EqualEqual_StrStr` (`self.GetWidgetName` _array_element) (`self.CurrentWidget`))))
  (return))

(fn `UnbindAllFinishAnim`
  (params (Widget :type "/Game/Blueprints/Widgets/Core/WBP_UserWidget Object Reference"))
  (clear `/Game/Blueprints/Widgets/Core/WBP_UserWidget.AppearFinish` Widget)
  (clear `/Game/Blueprints/Widgets/Core/WBP_UserWidget.DisapearFinish` Widget)
  (return))

(fn `UserConstructionScript`)