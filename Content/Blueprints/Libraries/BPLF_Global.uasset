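; Global helper library for debug printing, UI utilities, player controller access, language lookup and applying game settings.
; ApplySettings fans out to audio sound-mix overrides, Enhanced Input keybinds, video quality via GameUserSettings and console commands, culture, and controls.
; Move rebinding identifies each IA_Move direction by its modifiers, then swaps the key on matching mappings.
; UI helpers build per-state button styles, detect mouse movement, blend three colors and pick widget ZIndex from display names.
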(fn `ApplyAudio`
  (params (Settings :type "/Game/Classes/Structures/Settings/S_AudioSettings Structure"))
  (bind (_mastervolume _musicvolume _sfxvolume _voicevolume) (break `/Game/Classes/Structures/Settings/S_AudioSettings` Settings))
  (for (_array_element _array_index) (`|MakeArray` _mastervolume _musicvolume _sfxvolume _voicevolume)
    (`GameplayStatics.SetSoundMixClassOverride` null (select `int` _array_index :`0` "/Game/Resources/Sounds/Classes/MasterMix.MasterMix" :`1` "/Game/Resources/Sounds/Classes/MusicMix.MusicMix" :`2` "/Game/Resources/Sounds/Classes/SFXMix.SFXMix" :`3` "/Game/Resources/Sounds/Classes/VoiceMix.VoiceMix" :!type "SoundMix Object Reference") (select `int` _array_index :`0` "/Engine/EngineSounds/Master.Master" :`1` "/Engine/EngineSounds/Music.Music" :`2` "/Engine/EngineSounds/SFX.SFX" :`3` "/Engine/EngineSounds/Voice.Voice" :!type "SoundClass Object Reference") (`KismetMathLibrary.MapRangeClamped` _array_element 0.0 100.0 0.0 1.0) 1.0 0.0))
  (return))

(fn `ApplyControls`
  (params (Settings :type "/Game/Classes/Structures/Settings/S_ControlsSettings Structure"))
  (bind (_mappingcontext _crouch _interact _jump _pause _sprint) (break `/Game/Classes/Structures/Settings/S_ControlsSettings` Settings))
  (for (_array_element _array_index) (`|MakeArray` _crouch _interact _jump _pause _sprint)
    (bind _output (`|GetArrayItem` (`|MakeArray` "/Game/Inputs/Actions/Movement/IA_Crouch.IA_Crouch" "/Game/Inputs/Actions/IA_Interact.IA_Interact" "/Game/Inputs/Actions/Movement/IA_Jump.IA_Jump" "/Game/Inputs/Actions/IA_Pause.IA_Pause" "/Game/Inputs/Actions/Movement/IA_Sprint.IA_Sprint" :!type "InputAction Object Reference") _array_index))
    (`InputMappingContext.UnmapAllKeysFromAction` _mappingcontext _output)
    (`InputMappingContext.MapKey` _mappingcontext _output _array_element))
  (return))

(fn `ApplyGameplay`
  (params (Settings :type "/Game/Classes/Structures/Settings/S_GameplaySettings Structure"))
  (`KismetInternationalizationLibrary.SetCurrentCulture` (`self.GetLanguageValue` (`.GameLanguage_8_540F765A401B25283424C8A6A272EA37` (break `/Game/Classes/Structures/Settings/S_GameplaySettings` Settings))) true)
  (return))

(fn `ApplyKeybinds`
  (params (Settings :type "/Game/Classes/Structures/Settings/S_KeybindsSettings Structure"))
  (locals (MoveMappings :type "Map of String to EnhancedActionKeyMapping Structure"))
  (bind (_mappingcontext _crouch _interact _jump _movedown _moveleft _moveright _moveup _pause _sprint) (break `/Game/Classes/Structures/Settings/S_KeybindsSettings` Settings))
  (`BlueprintMapLibrary.Map_Clear` (`local.MoveMappings`))
  (for _array_element (`InputMappingContext.Mappings` _mappingcontext)
    (bind ((`Modifiers` _modifiers) (`Action` _action)) (break `EnhancedActionKeyMapping` _array_element))
    (if (`KismetStringLibrary.EqualEqual_StrStr` (`KismetSystemLibrary.GetDisplayName` _action) "IA_Move")
      (`BlueprintMapLibrary.Map_Add` (`local.MoveMappings`) (select `int` (`KismetArrayLibrary.Array_Length` _modifiers) :`0` "Move Right" :`1` (`KismetMathLibrary.SelectString` "Move Left" "Move Up" (`KismetStringLibrary.EqualEqual_StrStr` (`KismetSystemLibrary.GetDisplayName` (`|GetArrayItem` _modifiers)) "Negate")) :`2` "Move Down") _array_element)))
  (for (_array_element_2 _array_index) (`|MakeArray` _movedown _moveleft _moveright _moveup)
    (for _array_element_3 (`InputMappingContext.Mappings` _mappingcontext)
      (bind ((`Modifiers` _modifiers_2) (`Action` _action_2)) (break `EnhancedActionKeyMapping` _array_element_3))
      (if (== _action_2 "/Game/Inputs/Actions/Movement/IA_Move.IA_Move")
        (bind ((`Modifiers` _modifiers_3)) (break `EnhancedActionKeyMapping` (`BlueprintMapLibrary.Map_Find` (`local.MoveMappings`) (`|GetArrayItem` (`|MakeArray` "Move Down" "Move Left" "Move Right" "Move Up") _array_index))))
        (if (== (`KismetArrayLibrary.Array_Length` _modifiers_2) (`KismetArrayLibrary.Array_Length` _modifiers_3))
          (for (_array_element_4 _array_index_2) _modifiers_2
            (if (== _array_element_4 (`|GetArrayItem` _modifiers_3 _array_index_2))
              _))
          (setmembers `EnhancedActionKeyMapping` :`StructRef` _array_element_3 :`Key` _array_element_2)
          (`self.Print` "NewEnumerator4" "Find One !")))))
  (for (_array_element_5 _array_index_3) (`|MakeArray` _crouch _interact _jump _pause _sprint)
    (bind _output (`|GetArrayItem` (`|MakeArray` "/Game/Inputs/Actions/Movement/IA_Crouch.IA_Crouch" "/Game/Inputs/Actions/IA_Interact.IA_Interact" "/Game/Inputs/Actions/Movement/IA_Jump.IA_Jump" "/Game/Inputs/Actions/IA_Pause.IA_Pause" "/Game/Inputs/Actions/Movement/IA_Sprint.IA_Sprint" :!type "InputAction Object Reference") _array_index_3))
    (`InputMappingContext.UnmapAllKeysFromAction` _mappingcontext _output)
    (`InputMappingContext.MapKey` _mappingcontext _output _array_element_5))
  (return))

(fn `ApplySettings`
  (params (Settings :type "/Game/Classes/Structures/Settings/S_Settings Structure"))
  (bind (_audio _keybinds _video _gameplay _controls) (break `/Game/Classes/Structures/Settings/S_Settings` Settings))
  (`self.ApplyAudio` _audio)
  (`self.ApplyKeybinds` _keybinds)
  (`self.ApplyVideo` _video)
  (`self.ApplyGameplay` _gameplay)
  (`self.ApplyControls` _controls)
  (return))

(fn `ApplyVideo`
  (params (Settings :type "/Game/Classes/Structures/Settings/S_VideoSettings Structure"))
  (bind (_texturequality _visualeffectquality _viewdistancequality _antialiasingquality _postprocessingquality _shadowquality _shadingquality _foliagequality _reflectionquality _volumetricfogquality _frameratelimit _screenresolution _vsyncenabled _fullscreenmode) (break `/Game/Classes/Structures/Settings/S_VideoSettings` Settings))
  (bind _returnvalue (`GameUserSettings.GetGameUserSettings`))
  (`GameUserSettings.SetTextureQuality` _returnvalue _texturequality)
  (`GameUserSettings.SetVisualEffectQuality` _returnvalue _visualeffectquality)
  (`GameUserSettings.SetViewDistanceQuality` _returnvalue _viewdistancequality)
  (`GameUserSettings.SetAntiAliasingQuality` _returnvalue _antialiasingquality)
  (`GameUserSettings.SetPostProcessingQuality` _returnvalue _postprocessingquality)
  (`GameUserSettings.SetShadowQuality` _returnvalue _shadowquality)
  (`GameUserSettings.SetShadingQuality` _returnvalue _shadingquality)
  (`GameUserSettings.SetFoliageQuality` _returnvalue _foliagequality)
  (`GameUserSettings.SetFrameRateLimit` _returnvalue _frameratelimit)
  (`GameUserSettings.SetScreenResolution` _returnvalue _screenresolution)
  (`GameUserSettings.SetVSyncEnabled` _returnvalue _vsyncenabled)
  (`GameUserSettings.SetFullscreenMode` _returnvalue _fullscreenmode)
  (`GameUserSettings.ApplySettings` _returnvalue false)
  (`KismetSystemLibrary.ExecuteConsoleCommand` null (`KismetStringLibrary.Concat_StrStr` "sg.ReflectionQuality " (`KismetStringLibrary.Conv_IntToString` _reflectionquality)) null)
  (`KismetSystemLibrary.ExecuteConsoleCommand` null (`KismetStringLibrary.Concat_StrStr` "r.VolumetricFog.GridPixelSize " (select `int` (- _volumetricfogquality 1) :`0` "32" :`1` "16" :`2` "8" :`3` "4")) null)
  (return))

(fn `DisplayWidget`
  (params (Widget :type "UserWidget Object Reference") (`Display?` :type Boolean))
  (if `Display?`
    (`UserWidget.AddToViewport` Widget (`KismetMathLibrary.SelectInt` -1 0 (`KismetStringLibrary.EqualEqual_StrStr` (`KismetStringLibrary.Split` (`.RightS` (`KismetStringLibrary.Split` (`KismetSystemLibrary.GetDisplayName` Widget) "_")) "_") "BackgroundBlurred")))
    (else
      (`Widget.RemoveFromParent` Widget))))

(fn `GetButtonStyles`
  (params (Button :type "Button Object Reference"))
  (returns (Default :type "ButtonStyle Structure") (Normal :type "ButtonStyle Structure") (Hover :type "ButtonStyle Structure") (Pressed :type "ButtonStyle Structure"))
  (bind (_widgetstyle_normal _widgetstyle_hovered _widgetstyle_pressed _widgetstyle_disabled _widgetstyle_normalforeground _widgetstyle_hoveredforeground _widgetstyle_pressedforeground _widgetstyle_disabledforeground _widgetstyle_normalpadding _widgetstyle_pressedpadding _widgetstyle_pressedslatesound _widgetstyle_hoveredslatesound) (break `ButtonStyle` (`Button.WidgetStyle` Button)))
  (return (make `ButtonStyle` _widgetstyle_normal _widgetstyle_hovered _widgetstyle_pressed _widgetstyle_disabled _widgetstyle_normalforeground _widgetstyle_hoveredforeground _widgetstyle_pressedforeground _widgetstyle_disabledforeground _widgetstyle_normalpadding _widgetstyle_pressedpadding _widgetstyle_pressedslatesound _widgetstyle_hoveredslatesound) (make `ButtonStyle` _widgetstyle_normal _widgetstyle_normal _widgetstyle_normal _widgetstyle_disabled _widgetstyle_normalforeground _widgetstyle_normalforeground _widgetstyle_normalforeground _widgetstyle_disabledforeground _widgetstyle_normalpadding _widgetstyle_pressedpadding _widgetstyle_pressedslatesound _widgetstyle_hoveredslatesound) (make `ButtonStyle` _widgetstyle_hovered _widgetstyle_hovered _widgetstyle_hovered _widgetstyle_disabled _widgetstyle_hoveredforeground _widgetstyle_hoveredforeground _widgetstyle_hoveredforeground _widgetstyle_disabledforeground _widgetstyle_normalpadding _widgetstyle_pressedpadding _widgetstyle_pressedslatesound _widgetstyle_hoveredslatesound) (make `ButtonStyle` _widgetstyle_pressed _widgetstyle_pressed _widgetstyle_pressed _widgetstyle_disabled _widgetstyle_pressedforeground _widgetstyle_pressedforeground _widgetstyle_pressedforeground _widgetstyle_disabledforeground _widgetstyle_normalpadding _widgetstyle_pressedpadding _widgetstyle_pressedslatesound _widgetstyle_hoveredslatesound)))

(fn `GetController`
  (returns (Controller :type "/Game/Blueprints/Core/BPC_Player Object Reference"))
  (bind _asbpc_player (cast `/Game/Blueprints/Core/BPC_Player` (`GameplayStatics.GetPlayerController` null))
    (:`then`
      (return _asbpc_player))
    (:`CastFailed`
      (`self.Print` "NewEnumerator1" "-------------- CAST FAILED ------------------"))))

(fn `GetLanguageByString`
  (params (Value :type String))
  (returns (Language :type "/Game/Classes/Enums/E_Languages Enum"))
  (bind _enumvalue (foreach `/Game/Classes/Enums/E_Languages` false)
    (:`LoopBody`
      (if (`KismetStringLibrary.EqualEqual_StrStr` (`|GetEnumeratorNameAsString` _enumvalue) Value)
        (return _enumvalue)))
    (:`then`
      (return "NewEnumerator0"))))

(fn `GetLanguageValue`
  (params (Key :type "/Game/Classes/Enums/E_Languages Enum" :default "NewEnumerator0"))
  (returns (Value :type String))
  (bind _returnvalue (`DataTableFunctionLibrary.GetDataTableColumnAsString` "/Game/Blueprints/Data/DT_PlaystationButtons.DT_PlaystationButtons" "Key"))
  (bind _returnvalue_2 (`|GetDataTableRow` "/Game/Blueprints/Data/DT_LanguagesValues.DT_LanguagesValues" (`KismetStringLibrary.Conv_StringToName` (`KismetStringLibrary.Conv_IntToString` (`KismetArrayLibrary.Array_Find` _returnvalue (`|GetEnumeratorNameAsString` Key)))))
    (:`then`
      (return (`.Value_5_D044D81846B7C0B2593176971606ED4B` (break `/Game/Classes/Structures/S_LanguageEnumValues` _returnvalue_2))))
    (:`RowNotFound`
      (return "en"))))

(fn `Lerp3Color`
  (params (Colors :type "Array of LinearColor Structure") (Alpha :type "Float (double-precision)") (Interval :type "FloatInterval Structure"))
  (returns (`Output Color` :type "LinearColor Structure"))
  (bind (_min _max) (break `FloatInterval` Interval))
  (bind _output (`|GetArrayItem` Colors 1))
  (bind _returnvalue (/ (* (- Alpha _min) 100.0) (* (- _max _min) 100.0)))
  (bind _returnvalue_2 (* _returnvalue 2.0))
  (return (`KismetMathLibrary.SelectColor` (`KismetMathLibrary.LinearColorLerp` (`|GetArrayItem` Colors) _output _returnvalue_2) (`KismetMathLibrary.LinearColorLerp` _output (`|GetArrayItem` Colors 2) _returnvalue_2) (>= _returnvalue 0.5))))

(fn `MouseMoves?`
  (params (OldMousePos :type "Vector2D Structure (by ref)"))
  (returns (`IsMoving?` :type Boolean))
  (locals (Flexibility :type "Float (double-precision)" :default 10.0) (`IsMouseMoving?` :type Boolean))
  (bind (_x _y) (`KismetMathLibrary.BreakVector2D` OldMousePos))
  (bind _returnvalue (`WidgetLayoutLibrary.GetMousePositionOnViewport` null))
  (set `local.IsMouseMoving?` (>= (+ (`KismetMathLibrary.Abs` (- _x (`KismetMathLibrary.BreakVector2D` _returnvalue))) (`KismetMathLibrary.Abs` (- _y (`.Y` (`KismetMathLibrary.BreakVector2D` _returnvalue))))) (`local.Flexibility`)))
  (`KismetMathLibrary.Set2D` (`local.OldMousePos`) (`KismetMathLibrary.BreakVector2D` _returnvalue) (`.Y` (`KismetMathLibrary.BreakVector2D` _returnvalue)))
  (return (`local.IsMouseMoving?`)))

(fn `Print`
  (params (Type :type "/Game/Classes/Enums/E_PrintTypes Enum" :default "NewEnumerator0") (Message :type String :default "Message") (`Duration (in sec)` :type "Float (double-precision)" :default 2.0))
  (`KismetSystemLibrary.PrintString` null (select `bool` (`|EnumInequality` Type "NewEnumerator3") :`false` (`local.Message`) :`true` (`KismetStringLibrary.Concat_StrStr` "[" (`|GetEnumeratorNameAsString` (`local.Type`)) "]" (`local.Message`))) true true (select `/Game/Classes/Enums/E_PrintTypes` (`local.Type`) :`NewEnumerator0` (struct :`R` 1.0 :`A` 1.0) :`NewEnumerator1` (struct :`R` 1.0 :`G` 1.0 :`A` 1.0) :`NewEnumerator2` (struct :`G` 1.0 :`B` 1.0 :`A` 1.0) :`NewEnumerator4` (struct :`G` 1.0 :`B` 0.003 :`A` 1.0) :`NewEnumerator3` (struct :`R` 1.0 :`G` 1.0 :`B` 1.0 :`A` 1.0) :!type "LinearColor Structure") (`local.Duration (in sec)`)))