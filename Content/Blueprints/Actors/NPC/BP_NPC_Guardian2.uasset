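; Guardian NPC actor that offers an interaction prompt and fires a horror event when spoken to.
; A box trigger creates the NPC interaction widget when a HorrorEngineCharacter enters and removes it on any end overlap, without a cast check.
; Speak forwards to StartSpeaking, which runs HorrorEventCheck, while StopSpeaking is empty.
; The construction script runs the parent's, then HMDefaultConstructions with the CreateNewHorrorEvent setting.
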(event `StartSpeaking`
  (`self.HorrorEventCheck` "NewEnumerator3"))

(event `StopSpeaking`)

(event `self.Box.OnComponentBeginOverlap`
  (params (OverlappedComponent :type "PrimitiveComponent Object Reference") (OtherActor :type "Actor Object Reference") (OtherComp :type "PrimitiveComponent Object Reference") (OtherBodyIndex :type Integer) (bFromSweep :type Boolean) (SweepResult :type "HitResult Structure (by ref)"))
  (cast `/Game/HorrorEngine/Blueprints/Core/HorrorEngineCharacter` OtherActor)
  (bind _returnvalue (`|CreateWidget` "/Game/Blueprints/Widgets/Components/WBP_NPC_Interaction.WBP_NPC_Interaction_C"))
  (`UserWidget.AddToViewport` _returnvalue 0)
  (set `self.Widget` _returnvalue))

(event `self.Box.OnComponentEndOverlap`
  (params (OverlappedComponent :type "PrimitiveComponent Object Reference") (OtherActor :type "Actor Object Reference") (OtherComp :type "PrimitiveComponent Object Reference") (OtherBodyIndex :type Integer))
  (`Widget.RemoveFromParent` (`self.Widget`)))

(event `/Game/Blueprints/Actors/NPC/BPI_NPC_Interface.Speak`
  (`self.StartSpeaking`))

(fn `UserConstructionScript`
  (`parent.UserConstructionScript`)
  (`/Game/HorrorEngine/Blueprints/Core/HorrorEngineMacros.HM_DefaultConstructions` (`self.CreateNewHorrorEvent`)))