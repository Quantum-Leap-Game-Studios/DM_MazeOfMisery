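; Elevator door actor that acts as a level transition in the prison environment.
; On BeginPlay it caches both door transforms and, after a short delay, slides the doors apart along relative X using a timeline.
; Any overlap with the trigger box closes them once via a second timeline, provided the soft Level reference is valid.
; When closing finishes, it opens that level.
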(event `self.ReceiveBeginPlay`
  (set `self.Rightdoor_pos` (`SceneComponent.GetRelativeTransform` (`self.RightDoor`)))
  (set `self.NewVar` (`SceneComponent.GetRelativeTransform` (`self.LeftDoor`)))
  (`KismetSystemLibrary.Delay` 1.0)
  (`self.Open Door`))

(event `Open Door`
  (bind _newvar (`self.NewVar`))
  (bind _rightdoor_pos (`self.Rightdoor_pos`))
  (bind (_direction _transition) (`Timeline|Timeline` :!via `PlayFromStart`)
    (:`Update`
      (bind _returnvalue (`KismetMathLibrary.Lerp` 0.0 200.0 _transition))
      (`SceneComponent.K2_SetRelativeTransform` (`self.RightDoor`) (`KismetMathLibrary.MakeTransform` (`KismetMathLibrary.MakeVector` (- (.x (.location _rightdoor_pos)) _returnvalue) (.y (.location _rightdoor_pos)) (.z (.location _rightdoor_pos))) (.rotation _rightdoor_pos) (.scale _rightdoor_pos)) false false)
      (`SceneComponent.K2_SetRelativeTransform` (`self.LeftDoor`) (`KismetMathLibrary.MakeTransform` (`KismetMathLibrary.MakeVector` (+ (.x (.location _newvar)) _returnvalue) (.y (.location _newvar)) (.z (.location _newvar))) (.rotation _newvar) (.scale _newvar)) false false))))

(event `CloseDoors`
  (bind _level (`self.Level`))
  (bind _rightdoor_pos (`self.Rightdoor_pos`))
  (bind _newvar (`self.NewVar`))
  (if (and (not (`self.IsClose`)) (`KismetSystemLibrary.IsValidSoftObjectReference` (`self.Level`)))
    (bind (_direction _transition) (`Timeline|Timeline_0` :!via `PlayFromStart`)
      (:`Update`
        (bind _returnvalue (`KismetMathLibrary.Lerp` 0.0 200.0 _transition))
        (`SceneComponent.K2_SetRelativeTransform` (`self.RightDoor`) (`KismetMathLibrary.MakeTransform` (`KismetMathLibrary.MakeVector` (+ _returnvalue (- (.x (.location _rightdoor_pos)) 200.0)) (.y (.location _rightdoor_pos)) (.z (.location _rightdoor_pos))) (.rotation _rightdoor_pos) (.scale _rightdoor_pos)) false false)
        (`SceneComponent.K2_SetRelativeTransform` (`self.LeftDoor`) (`KismetMathLibrary.MakeTransform` (`KismetMathLibrary.MakeVector` (- (+ (.x (.location _newvar)) 200.0) _returnvalue) (.y (.location _newvar)) (.z (.location _newvar))) (.rotation _newvar) (.scale _newvar)) false false))
      (:`Finished`
        (if (`KismetSystemLibrary.IsValidSoftObjectReference` _level)
          (`GameplayStatics.OpenLevelBySoftObjectPtr` _level))))))

(event `self.TriggerBox.OnComponentBeginOverlap`
  (params (OverlappedComponent :type "PrimitiveComponent Object Reference") (OtherActor :type "Actor Object Reference") (OtherComp :type "PrimitiveComponent Object Reference") (OtherBodyIndex :type Integer) (bFromSweep :type Boolean) (SweepResult :type "HitResult Structure (by ref)"))
  (`self.CloseDoors`)
  (set `self.IsClose` true))

(fn `UserConstructionScript`)