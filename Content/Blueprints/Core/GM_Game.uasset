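; GM_Game is the gameplay Blueprint, apparently a game mode, that hides the mouse cursor on BeginPlay and handles pausing.
; Its Pause/UnpauseGame event toggles the paused state, creating a blurred background widget and then a pause widget in the viewport when pausing.
; The unpause branch only clears the paused state and does not remove either widget itself.
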(event `self.ReceiveBeginPlay`
  (set `PlayerController.bShowMouseCursor` false (`GameplayStatics.GetPlayerController` 0)))

(event `Pause / Unpause Game`
  (if (`GameplayStatics.IsGamePaused`)
    (`GameplayStatics.SetGamePaused` false)
    (else
      (`GameplayStatics.SetGamePaused` true)
      ;[0.2002 0.2934 0.0758] Blurred Background
      (bind _returnvalue (`|CreateWidget` "/Game/Blueprints/Widgets/Components/WBP_BackgroundBlurred.WBP_BackgroundBlurred_C"))
      (`UserWidget.AddToViewport` _returnvalue 0)
      ;[0.2002 0.2934 0.0758] Pause Widget
      (bind _returnvalue_2 (`|CreateWidget` "/Game/Blueprints/Widgets/WBP_Pause.WBP_Pause_C"))
      (`UserWidget.AddToViewport` _returnvalue_2 0))))

(fn `UserConstructionScript`)