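; Global Blueprint function library of shared debug, input and UI helpers.
; Print shows color-coded messages by type, MouseMoves detects cursor movement against a tolerance while updating the stored position, and GetController returns the player controller cast to BPC_Player, warning on failure.
; GetButtonStyles derives default, normal, hover and pressed style variants from a button.
; DisplayWidget adds or removes widgets, parsing the display name to put blurred backgrounds behind others.
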(fn `DisplayWidget`
  (params (Widget :type "UserWidget Object Reference") (`Display?` :type Boolean))
  (if `Display?`
    (`UserWidget.AddToViewport` Widget (`KismetMathLibrary.SelectInt` -1 0 (`KismetStringLibrary.EqualEqual_StrStr` (`KismetStringLibrary.Split` (`.RightS` (`KismetStringLibrary.Split` (`KismetSystemLibrary.GetDisplayName` Widget) "_")) "_") "BackgroundBlurred")))
    (else
      (`Widget.RemoveFromParent` Widget))))

(fn `GetButtonStyles`
  (params (Button :type "Button Object Reference"))
  (returns (Default :type "ButtonStyle Structure") (Normal :type "ButtonStyle Structure") (Hover :type "ButtonStyle Structure") (Pressed :type "ButtonStyle Structure"))
  (bind (_widgetstyle_normal _widgetstyle_hovered _widgetstyle_pressed _widgetstyle_disabled _widgetstyle_normalforeground _widgetstyle_hoveredforeground _widgetstyle_pressedforeground _widgetstyle_disabledforeground _widgetstyle_normalpadding _widgetstyle_pressedpadding _widgetstyle_pressedslatesound _widgetstyle_hoveredslatesound) (break `ButtonStyle` (`Button.WidgetStyle` Button)))
  (return (make `ButtonStyle` _widgetstyle_normal _widgetstyle_hovered _widgetstyle_pressed _widgetstyle_disabled _widgetstyle_normalforeground _widgetstyle_hoveredforeground _widgetstyle_pressedforeground _widgetstyle_disabledforeground _widgetstyle_normalpadding _widgetstyle_pressedpadding _widgetstyle_pressedslatesound _widgetstyle_hoveredslatesound) (make `ButtonStyle` _widgetstyle_normal _widgetstyle_normal _widgetstyle_normal _widgetstyle_disabled _widgetstyle_normalforeground _widgetstyle_normalforeground _widgetstyle_normalforeground _widgetstyle_disabledforeground _widgetstyle_normalpadding _widgetstyle_pressedpadding _widgetstyle_pressedslatesound _widgetstyle_hoveredslatesound) (make `ButtonStyle` _widgetstyle_hovered _widgetstyle_hovered _widgetstyle_hovered _widgetstyle_disabled _widgetstyle_hoveredforeground _widgetstyle_hoveredforeground _widgetstyle_hoveredforeground _widgetstyle_disabledforeground _widgetstyle_normalpadding _widgetstyle_pressedpadding _widgetstyle_pressedslatesound _widgetstyle_hoveredslatesound) (make `ButtonStyle` _widgetstyle_pressed _widgetstyle_pressed _widgetstyle_pressed _widgetstyle_disabled _widgetstyle_pressedforeground _widgetstyle_pressedforeground _widgetstyle_pressedforeground _widgetstyle_disabledforeground _widgetstyle_normalpadding _widgetstyle_pressedpadding _widgetstyle_pressedslatesound _widgetstyle_hoveredslatesound)))

(fn `GetController`
  (returns (Controller :type "/Game/Blueprints/Core/BPC_Player Object Reference"))
  (bind _asbpc_player (cast `/Game/Blueprints/Core/BPC_Player` (`GameplayStatics.GetPlayerController` null))
    (:`then`
      (return _asbpc_player))
    (:`CastFailed`
      (`self.Print` "NewEnumerator1" "-------------- CAST FAILED ------------------"))))

(fn `MouseMoves?`
  (params (OldMousePos :type "Vector2D Structure (by ref)"))
  (returns (`IsMoving?` :type Boolean))
  (locals (Flexibility :type "Float (double-precision)" :default 10.0) (`IsMouseMoving?` :type Boolean))
  (bind (_x _y) (`KismetMathLibrary.BreakVector2D` OldMousePos))
  (bind _returnvalue (`WidgetLayoutLibrary.GetMousePositionOnViewport` null))
  (set `local.IsMouseMoving?` (>= (+ (`KismetMathLibrary.Abs` (- _x (`KismetMathLibrary.BreakVector2D` _returnvalue))) (`KismetMathLibrary.Abs` (- _y (`.Y` (`KismetMathLibrary.BreakVector2D` _returnvalue))))) (`local.Flexibility`)))
  (`KismetMathLibrary.Set2D` (`local.OldMousePos`) (`KismetMathLibrary.BreakVector2D` _returnvalue) (`.Y` (`KismetMathLibrary.BreakVector2D` _returnvalue)))
  (return (`local.IsMouseMoving?`)))

(fn `Print`
  (params (Type :type "/Game/Classes/Enums/E_PrintTypes Enum" :default "NewEnumerator0") (Message :type String :default "Message") (`Duration (in sec)` :type "Float (double-precision)" :default 2.0))
  (`KismetSystemLibrary.PrintString` null (select `bool` (`|EnumInequality` Type "NewEnumerator3") :`false` (`local.Message`) :`true` (`KismetStringLibrary.Concat_StrStr` "[" (`|GetEnumeratorNameAsString` (`local.Type`)) "]" (`local.Message`))) true true (select `/Game/Classes/Enums/E_PrintTypes` (`local.Type`) :`NewEnumerator0` (struct :`R` 1.0 :`A` 1.0) :`NewEnumerator1` (struct :`R` 1.0 :`G` 1.0 :`A` 1.0) :`NewEnumerator2` (struct :`G` 1.0 :`B` 1.0 :`A` 1.0) :`NewEnumerator4` (struct :`G` 1.0 :`B` 0.003 :`A` 1.0) :`NewEnumerator3` (struct :`R` 1.0 :`G` 1.0 :`B` 1.0 :`A` 1.0) :!type "LinearColor Structure") (`local.Duration (in sec)`)))